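; MedievalPot is a cooking-project pot actor that shows name and interact widgets when its IsLooking event fires.
; The event calls WidgetLookAtCamera, which makes both widgets visible and rotates each toward the player camera once per call.
; After a five-second delay, the event hides both widgets again.
; BeginPlay also enables mouse-over events on the first player controller.
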(event `self.ReceiveBeginPlay`
  (set `PlayerController.bEnableMouseOverEvents` true (`GameplayStatics.GetPlayerController` 0)))

(event `IsLooking_Event`
  (bind _array (`|MakeArray` (`self.NameWidget`) (`self.InteractWidget`)))
  (`self.WidgetLookAtCamera` _array)
  (`KismetSystemLibrary.Delay` 5.0)
  (for _array_element _array
    (`SceneComponent.SetVisibility` _array_element false false)))

(fn `UserConstructionScript`)

(fn `WidgetLookAtCamera`
  (params (Widget :type "Array of WidgetComponent Object Reference"))
  (returns (OutWidget :type "WidgetComponent Object Reference"))
  (for _array_element Widget
    (`SceneComponent.SetVisibility` _array_element true false)
    (`SceneComponent.K2_SetWorldRotation` _array_element (`KismetMathLibrary.FindLookAtRotation` (`SceneComponent.K2_GetComponentLocation` _array_element) (`SceneComponent.K2_GetComponentLocation` (`PlayerCameraManager.TransformComponent` (`GameplayStatics.GetPlayerCameraManager` 0)))) false false))
  (return _array_element))